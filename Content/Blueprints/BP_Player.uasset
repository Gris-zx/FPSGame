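; Player character Blueprint with sprint, a blink dash, an HP bar and death handling.
; Left Shift sprints when unlocked; a quick second press, if blink is unlocked, plays a timeline that sweeps the actor forward and widens camera FOV.
; Tick watches HP and, near zero, stops movement, then after a delay pauses the game and shows the GameEnd widget with cursor.
; Test keys P, O and I unlock sprint, unlock blink and deal damage.
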(event EventBeginPlay
  ;[1 1 1] 血量
  (bind _returnvalue (UserInterface|CreateWidget "/Game/UI/HP_Bar.HP_Bar_C"))
  (Utilities|IsValid _returnvalue
    (:Is%20Valid
      (UserInterface|Viewport|AddtoViewport _returnvalue 0))))

(event EventTick
  (params (DeltaSeconds :type Float%20%28single-precision%29))
  (bind _returnvalue (Game|GetPlayerCharacter 0))
  (bind _charactermovement (Variables|/Script/Engine.Character|GetCharacterMovement _returnvalue))
  (Utilities|FlowControl|Sequence
    (:then_0
      (if (<= (Variables|Default|GetHP_recent) 2.0)
        (Variables|Default|Setisdie? true)))
    (:then_1
      (if (Variables|Default|Getisdie?)
        (Variables|/Script/Engine.CharacterMovementComponent|SetMaxWalkSpeed _charactermovement 0.0)
        (Variables|/Script/Engine.CharacterMovementComponent|SetRotationRate _charactermovement "0, 0, 0")
        (Utilities|FlowControl|Delay 0.5)
        (Game|SetGamePaused true)
        (bind _returnvalue_2 (UserInterface|CreateWidget "/Game/UI/GameEnd.GameEnd_C"))
        (UserInterface|Viewport|AddtoViewport _returnvalue_2 0)
        (Variables|/Script/Engine.PlayerController|SetbShowMouseCursor (Game|GetPlayerController 0) true)))))

(event Input|KeyboardEvents|LeftShift
  (params (Key :type Key%20Structure :default "None"))
  (bind _returnvalue (Transformation|GetActorLocation))
  (bind _charactermovement (Variables|Character|GetCharacterMovement))
  (:Pressed
    (if (Variables|Default|Get加速可用)
      (Variables|/Script/Engine.CharacterMovementComponent|SetMaxWalkSpeed _charactermovement 1.2e+03)
      (Math|Integer|IncrementInt (Variables|Default|Get次数)
        (:%20%20
          (if (and (>= (Variables|Default|Get次数) 2) (Variables|Default|Get闪现可用))
            (bind _新建轨道_0 (Timeline|时间轴_0 PlayFromStart)
              (:Update
                (Transformation|SetActorLocation (Math|Vector|Lerp(Vector) _returnvalue (+ _returnvalue (* (Transformation|GetActorForwardVector) 5e+02)) _新建轨道_0) true false)
                (Camera|SetFieldOfView (Variables|Default|GetCameraComponent) (Math|Float|Lerp 8e+01 9e+01 _新建轨道_0)))))))))
  (:Released
    (Variables|/Script/Engine.CharacterMovementComponent|SetMaxWalkSpeed _charactermovement 6e+02)
    (Utilities|FlowControl|Delay 0.2)
    (Variables|Default|Set次数 0)))

(event Input|KeyboardEvents|O
  (params (Key :type Key%20Structure :default "None"))
  ;[1 1 1] 测试
  ;;[1 1 1] 测试
  (:Pressed
    (Variables|Default|Set闪现可用 true)))

(event Input|KeyboardEvents|I
  (params (Key :type Key%20Structure :default "None"))
  ;[1 1 1] 测试
  (:Pressed
    (Variables|Default|SetHP_recent (- (Variables|Default|GetHP_recent) 15.0))))

(event Input|KeyboardEvents|P
  (params (Key :type Key%20Structure :default "None"))
  ;[1 1 1] 测试
  ;;[1 1 1] 测试
  (:Pressed
    (Variables|Default|Set加速可用 true)))

(fn ConstructionScript)