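; BP_Guard is a guard character Blueprint that shows its awareness state and handles the end-of-mission presentation.
; On state change, it sets its WBP_GuardState widget component to a blank, question or exclamation mark for idle, suspicious or alerted.
; On mission completion, it shows WBP_GameOver with the success flag and blends the instigating player's camera to the first BP_SpectatingViewpoint found in the level.
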(event EventOnStateChanged
  (params (NewState :type EAIState%20Enum :default "Idle"))
  (bind _aswbp_guard_state (Utilities|Casting|CastToWBP_GuardState (UserInterface|GetUserWidgetObject (Variables|Default|GetWidget))))
  (Default|UpdateText _aswbp_guard_state (Utilities|Select :Index NewState :Idle "" :Suspicious "?" :Alerted "!")))

(event EventOnMissionCompleted
  (params (InstigatorPawn :type Pawn%20Object%20Reference) (bMissionSuccess :type Boolean))
  (Utilities|FlowControl|Sequence
    (:then_0
      (bind _returnvalue (UserInterface|CreateWidget "/Game/UI/WBP_GameOver.WBP_GameOver_C" 0 bMissionSuccess))
      (UserInterface|Viewport|AddtoViewport _returnvalue 0))
    (:then_1
      (bind _as玩家控制器 (Utilities|Casting|CastToPlayerController (Pawn|GetController InstigatorPawn)))
      (bind _outactors (Actor|GetAllActorsOfClass "/Game/Blueprints/BP_SpectatingViewpoint.BP_SpectatingViewpoint_C"))
      (Game|Player|SetViewTargetwithBlend _as玩家控制器 (Utilities|Array|Get(acopy) _outactors) 0.5 "VTBlend_Cubic" 0.0 false))))

(fn ConstructionScript)