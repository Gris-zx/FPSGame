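; BP_PropCar01 is a car prop pickup that grants BP_Player an acceleration skill.
; Entering its Box caches the player, shows an F-key prompt, enables input on the actor and opens a Gate.
; Pressing F while the Gate is open sets the player's 加速可用 flag and prints hold-Shift instructions.
; Leaving closes the Gate but calls EnableInput again, so only the Gate blocks the key.
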(event OnComponentBeginOverlap(Box)
  (params (OverlappedComponent :type Primitive%20Component%20Object%20Reference) (OtherActor :type Actor%20Object%20Reference) (OtherComp :type Primitive%20Component%20Object%20Reference) (OtherBodyIndex :type Integer) (bFromSweep :type Boolean) (SweepResult :type Hit%20Result%20Structure%20%28by%20ref%29))
  (bind _asbp_player (Utilities|Casting|CastToBP_Player OtherActor))
  (Development|PrintString "按F获取新技能加速！" true true "(R=1.000000,G=0.892658,B=0.062500,A=1.000000)")
  (Input|EnableInput (Game|GetPlayerController 0))
  (Utilities|FlowControl|Gate true) ; enters at Open
)

(event OnComponentEndOverlap(Box)
  (params (OverlappedComponent :type Primitive%20Component%20Object%20Reference) (OtherActor :type Actor%20Object%20Reference) (OtherComp :type Primitive%20Component%20Object%20Reference) (OtherBodyIndex :type Integer))
  (Utilities|Casting|CastToBP_Player OtherActor)
  (Input|EnableInput (Game|GetPlayerController 0))
  (Utilities|FlowControl|Gate true) ; enters at Close
)

(event EventBeginPlay)

(event Collision|EventActorBeginOverlap
  (params (OtherActor :type Actor%20Object%20Reference)))

(event EventTick
  (params (DeltaSeconds :type Float%20%28single-precision%29)))

(event Input|KeyboardEvents|F
  (params (Key :type Key%20Structure :default "None"))
  (:Pressed
    (Utilities|FlowControl|Gate true
      (:Exit
        (Variables|/Game/Blueprints/BP_Player.BP_Player_C|Set加速可用 (stale OnComponentBeginOverlap(Box) _asbp_player) true)
        (Development|PrintString "已获得加速技能！" true true "(R=0.850000,G=0.000000,B=0.000000,A=1.000000)")
        (Development|PrintString "按住\"Shift\"键加速！" true true "(R=0.000000,G=1.000000,B=0.144330,A=1.000000)" 1e+01)))))

(fn ConstructionScript)